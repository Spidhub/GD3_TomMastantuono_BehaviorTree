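; BP_Pnj is an AI-controlled NPC that fires projectiles at the player.
; Shoot decrements the Ammo blackboard key, spawns a BP_Projectile at the Muzzle and sends it at high speed toward the player pawn's current location.
; The Shooting flag stays true for a short delay after each shot, and no ammo check happens here.
; BeginPlay only casts the game mode, without using the result.
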(event `self.ReceiveBeginPlay`
  (cast `/Game/ThirdPerson/Blueprints/BP_ThirdPersonGameMode` (`GameplayStatics.GetGameMode`)))

(event `/Game/Exo_Behavior/BPI_Behave.Shoot`
  (bind _ammo (`self.Ammo`))
  (bind _returnvalue_location (`KismetMathLibrary.BreakTransform` (`SceneComponent.K2_GetComponentToWorld` (`self.muzzle`))))
  (bind _returnvalue (`AIBlueprintHelperLibrary.GetBlackboard` (`AIBlueprintHelperLibrary.GetAIController` self)))
  (`BlackboardComponent.SetValueAsInt` _returnvalue _ammo (- (`BlackboardComponent.GetValueAsInt` _returnvalue _ammo) 1))
  (set `self.Shooting?` true)
  (bind _returnvalue_2 (`|SpawnActorFromClass` "/Game/Exo_Behavior/BP_Projectile.BP_Projectile_C" (`KismetMathLibrary.MakeTransform` _returnvalue_location) "AlwaysSpawn" "MultiplyWithRoot" null null))
  (bind _projectilemovement (`/Game/Exo_Behavior/BP_Projectile.ProjectileMovement` _returnvalue_2))
  (set `MovementComponent.Velocity` (* (`KismetMathLibrary.Normal` (- (`self.K2_GetActorLocation` (`GameplayStatics.GetPlayerPawn` 0)) _returnvalue_location)) 8000.0) _projectilemovement)
  (`ActorComponent.Activate` _projectilemovement false)
  (`KismetSystemLibrary.Delay` 0.5)
  (set `self.Shooting?` false))

(fn `UserConstructionScript`)